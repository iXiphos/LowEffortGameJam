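; CactusGameMode is a game mode that ends the game when the player's CactusGunner character runs out of health.
; Every Tick it polls that character's Health and opens the EndScreen level once it reaches zero or below.
; The same Tick also re-applies pitch and yaw limits on the player camera manager to restrict the view.
; BeginPlay is labelled for game music but is empty.
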(event Custom|EndGameEvent
  ;[1 1 1] End Game stuff (Open End Level)
  (bind _ascactus_gunner (Utilities|Casting|CastToCactusGunner (Game|GetPlayerCharacter 0)))
  (bind _output_get (Variables|Default|SetRunning (<= (Variables|/Game/AidanFolder/Blueprints/CactusGunner.CactusGunner_C|GetHealth _ascactus_gunner) 0)))
  (if _output_get
    (Game|OpenLevel(byName) "EndScreen")))

(event EventBeginPlay
  ;[1 1 1] Add Game Music
)

(event EventTick
  (params (DeltaSeconds :type Float%20%28single-precision%29))
  (bind _returnvalue (Game|GetPlayerCameraManager 0))
  (CallFunction|EndGameEvent)
  (Variables|/Script/Engine.PlayerCameraManager|SetViewPitchMax _returnvalue 5e+01)
  (Variables|/Script/Engine.PlayerCameraManager|SetViewPitchMin _returnvalue -6e+01)
  (Variables|/Script/Engine.PlayerCameraManager|SetViewYawMax _returnvalue 45.0)
  (Variables|/Script/Engine.PlayerCameraManager|SetViewYawMin _returnvalue -45.0))

(fn ConstructionScript)