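; HUD Blueprint that draws the crosshair and the score on screen.
; On each DrawHUD event it draws the Reticle texture at a fixed size near screen center, using hard-coded pixel offsets that leave it slightly off-center horizontally.
; It then prints the Score value as enlarged text toward the top-left, positioned proportionally to screen size; nothing here updates that value.
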(event EventDrawHUD
  (params (SizeX :type Integer) (SizeY :type Integer))
  (Canvas|DrawTexture "/Game/Assets/Textures/Reticle.Reticle" (Math|Conversions|ToFloat(Integer) (+ (/ SizeX 2) -15)) (Math|Conversions|ToFloat(Integer) (+ (/ SizeY 2) -20)) 4e+01 4e+01 0.0 1.0 1.0 1.0 "(R=1.000000,G=1.000000,B=1.000000,A=1.000000)")
  (HUD|DrawText (Utilities|String|ToString(Integer) (Variables|Default|GetScore)) "(R=0,G=0,B=0,A=1)" (Math|Conversions|ToFloat(Integer) (/ SizeX 7)) (Math|Conversions|ToFloat(Integer) (/ SizeY 7)) 0 5.0 false))

(fn ConstructionScript)