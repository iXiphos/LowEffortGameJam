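; CactusGunner is a player-controlled gunner with mouse-look style axis rotation, an automatic cactus gun, timed reload and damage-reduced health.
; Fire input plays the looping gun animation and opens a Tick gate, throttled by a FireDelay flag and short Delay.
; Each shot spawns a Bullet with camera shake and sound, while a debug-drawn camera line trace separately applies damage to exact Enemy-class hits.
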(event EventTick
  (params (DeltaSeconds :type Float%20%28single-precision%29))
  (bind _camera (Variables|Camera|GetCamera))
  (bind _camera_2 (Variables|Camera|GetCamera))
  (bind _sphere (Variables|Default|GetSphere))
  (bind _returnvalue (Transformation|GetWorldLocation _sphere))
  (bind _returnvalue_2 (Transformation|GetWorldLocation _camera))
  (Utilities|FlowControl|Gate true
    (:Exit
      (if (Variables|Default|GetFireDelay)
        (Variables|Default|SetFireDelay false)
        (Math|Integer|CompareInt (Variables|Default|GetAmmoCount)
          (:>
            (Variables|Default|SetAmmoCount (- (Variables|Default|GetAmmoCount) 1))
            (Math|Integer|CompareInt (Variables|Default|GetAmmoCount)
              (:>
                (bind _outhit (Collision|LineTraceByChannel _returnvalue_2 (+ _returnvalue_2 (* (Math|Vector|GetForwardVector _camera) 1e+05)) "TraceTypeQuery1" false 0 "ForDuration" true "(R=1.000000,G=0.000000,B=0.000000,A=1.000000)" "(R=0.000000,G=1.000000,B=0.000000,A=1.000000)" 0.3))
                (Class|PlayerCameraManager|StartCameraShakefromSource (Game|GetPlayerCameraManager 0) "/Game/AidanFolder/Blueprints/CameraShake.CameraShake_C" 0 1.0 "CameraLocal" "0, 0, 0")
                (Audio|PlaySoundatLocation "/Game/AidanFolder/Blueprints/510278__tripjazz__bottle-opening.510278__tripjazz__bottle-opening" _returnvalue "0, 0, 0" 1.0 1.0 0.0 0 0 0)
                (Game|SpawnActorfromClass "/Game/AidanFolder/Blueprints/Bullet.Bullet_C" (Math|Transform|MakeTransform _returnvalue (Transformation|GetWorldRotation _camera_2) "0.100000,0.100000,0.100000") "Undefined" 0 (* (Math|Vector|GetForwardVector _camera_2) 7.5e+03) 0)
                (if (== (Utilities|GetClass (.HitActor (Collision|BreakHitResult _outhit))) "/Game/Blueprints/Enemy.Enemy_C")
                  (Game|Damage|ApplyDamage (.HitActor (Collision|BreakHitResult _outhit)) (Variables|Default|GetDamage) 0 0)))
              (:==
                (Audio|Components|Audio|Stop (Variables|Default|GetCactigun) :!label _label))
              (:<
                (goto _label)))))
        (else
          (Utilities|FlowControl|Delay 0.1)
          (Variables|Default|SetFireDelay true))))))

(event Game|Damage|EventAnyDamage
  (params (Damage :type Float%20%28single-precision%29) (DamageType :type Damage%20Type%20Object%20Reference) (InstigatedBy :type Controller%20Object%20Reference) (DamageCauser :type Actor%20Object%20Reference))
  (Development|PrintString (Utilities|String|ToString(Integer) (Variables|Default|GetHealth)))
  (Variables|Default|SetHealth (Math|Float|Truncate (- (Math|Conversions|ToFloat(Integer) (Variables|Default|GetHealth)) Damage))))

(event Input|ActionEvents|InputActionFire
  (params (Key :type Key%20Structure :default "None"))
  (bind _camera (Variables|Camera|GetCamera))
  (bind _camera_2 (Variables|Camera|GetCamera))
  (bind _sphere (Variables|Default|GetSphere))
  (bind _cactigun (Variables|Default|GetCactigun))
  (bind _returnvalue (Transformation|GetWorldLocation _sphere))
  (bind _returnvalue_2 (Transformation|GetWorldLocation _camera))
  (:Pressed
    (Math|Integer|CompareInt (Variables|Default|GetAmmoCount)
      (:>
        (Components|Animation|PlayAnimation _cactigun "/Game/Assets/Cactigun_Anim.Cactigun_Anim" true)
        (Utilities|FlowControl|Gate true) ; enters at Open
      )
      (:==
        (Audio|Components|Audio|Stop _cactigun :!label _label)
        (Utilities|FlowControl|Gate true) ; enters at Open
      )
      (:<
        (goto _label))))
  (:Released
    (Audio|Components|Audio|Stop _cactigun)
    (Utilities|FlowControl|Gate true) ; enters at Close
  ))

(event Input|ActionEvents|InputActionReload
  (params (Key :type Key%20Structure :default "None"))
  (:Pressed
    (Variables|Default|SetAmmoCount 0)
    (Audio|PlaySoundatLocation "/Game/Blueprints/Recording.Recording" "0, 0, 0" "0, 0, 0" 1.0 1.0 0.0 0 0 0)
    (Utilities|FlowControl|Delay (Variables|Default|GetReloadTime))
    (Variables|Default|SetAmmoCount (Variables|Default|GetAmmoTotal))))

(event Input|AxisEvents|InputAxisRotate_LeftRight
  (params (AxisValue :type Float%20%28single-precision%29))
  (Pawn|Input|AddControllerYawInput AxisValue))

(event Input|AxisEvents|InputAxisRotate_UpDown
  (params (AxisValue :type Float%20%28single-precision%29))
  (Pawn|Input|AddControllerPitchInput AxisValue))

(fn ConstructionScript)