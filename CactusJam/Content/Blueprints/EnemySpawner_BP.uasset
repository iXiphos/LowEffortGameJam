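; Enemy spawner actor that spawns an Enemy at its own transform on BeginPlay, then repeatedly on a timed interval.
; Tick accumulates delta time until it reaches TimeBetween, then resets the counter, prints a debug string and reuses the BeginPlay spawn node.
; An unconnected chain that would print and set the elapsed time to just under TimeBetween never runs.
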(event EventBeginPlay
  (Game|SpawnActorfromClass "/Game/Blueprints/Enemy.Enemy_C" (Transformation|GetActorTransform) "Undefined" 0 0))

(event Collision|EventActorBeginOverlap
  (params (OtherActor :type Actor%20Object%20Reference)))

(event EventTick
  (params (DeltaSeconds :type Float%20%28single-precision%29))
  (bind _output_get (Variables|Default|SetTimeElapsed (+ DeltaSeconds (Variables|Default|GetTimeElapsed))))
  (if (not (< _output_get (Variables|Default|GetTimeBetween)))
    (Variables|Default|SetTimeElapsed 0.0)
    (Development|PrintString "0")
    (Game|SpawnActorfromClass "/Game/Blueprints/Enemy.Enemy_C" (Transformation|GetActorTransform) "Undefined" 0 0)))

(fn ConstructionScript)